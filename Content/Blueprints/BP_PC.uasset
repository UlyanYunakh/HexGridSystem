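; BP_PC is a player controller that shows the mouse cursor on BeginPlay and provides a debug readout of tile distances.
; Its DistanceTo event measures the tile distance from the stored StartPoint to a given tile.
; It prints both tiles and the result on screen for a long duration, framed by separator lines.
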(event `self.ReceiveBeginPlay`
  (set `self.bShowMouseCursor` true))

(event `DistanceTo`
  (params (Other :type "HGS_Tile Structure"))
  (`KismetSystemLibrary.PrintString` "---------" true true (struct :`G` 0.66 :`B` 1.0 :`A` 1.0) 60.0)
  (`KismetSystemLibrary.PrintString` (`KismetStringLibrary.Concat_StrStr` "Distance between A(" (`HGS_Library.TileToSring` (`self.StartPoint`)) ") and B(" (`HGS_Library.TileToSring` Other) ") = " (`KismetStringLibrary.Conv_DoubleToString` (`HGS_Library.TileDistance` (`self.StartPoint`) Other))) true true (struct :`G` 0.66 :`B` 1.0 :`A` 1.0) 60.0)
  (`KismetSystemLibrary.PrintString` "---------" true true (struct :`G` 0.66 :`B` 1.0 :`A` 1.0) 60.0))

(fn `UserConstructionScript`)