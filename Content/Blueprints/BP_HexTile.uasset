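; BP_HexTile is a clickable hex tile actor that shows and prints debug information about its tile in the HGS grid.
; The construction script looks up the tile by the HGSActorSnap key and writes its coordinate and reference count to text components.
; Left-click prints the tile's neighbours.
; Right-click passes the tile to DistanceTo on BP_PC, the player controller.
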(event `self.ReceiveBeginPlay`
  (add `self.OnClicked` (delegate `OnClicked_Event`)))

(event `OnClicked_Event` :!signature `self.OnClicked`
  (params (TouchedActor :type "Actor Object Reference") (ButtonPressed :type "Key Structure" :default "None"))
  (bind _returnvalue (`HGS_Library.GetHGS` self))
  (`/Engine/EditorBlueprintResources/StandardMacros.IsValid` _returnvalue
    (:`Is Valid`
      (bind (_outtile _returnvalue_2) (`HGS_Data.GetTileByKey` _returnvalue (`HGS_ActorSnapComponent.TileKey` (`self.HGS_ActorSnap`))))
      (if _returnvalue_2
        (if (== ButtonPressed "LeftMouseButton")
          (`KismetSystemLibrary.PrintString` "------" true true (struct :`G` 0.66 :`B` 1.0 :`A` 1.0) 60.0)
          (for _array_element (`HGS_Data.GetNeighbours` _returnvalue _outtile)
            (`KismetSystemLibrary.PrintString` (`HGS_Library.TileToSring` _array_element) true true (struct :`G` 0.66 :`B` 1.0 :`A` 1.0) 60.0))
          (`KismetSystemLibrary.PrintString` (`KismetStringLibrary.Concat_StrStr` "--- Neighbours of " (`HGS_Library.TileToSring` _outtile) " ---") true true (struct :`G` 0.66 :`B` 1.0 :`A` 1.0) 90.0)
          (elif (== ButtonPressed "RightMouseButton")
            (bind _asbp_pc (cast `/Game/Blueprints/BP_PC` (`GameplayStatics.GetPlayerController` 0)))
            (`/Game/Blueprints/BP_PC.DistanceTo` _asbp_pc _outtile)))))))

(fn `UserConstructionScript`
  (bind _returnvalue (`HGS_Library.GetHGS` self))
  (`/Engine/EditorBlueprintResources/StandardMacros.IsValid` _returnvalue
    (:`Is Valid`
      (bind (_outtile _returnvalue_2) (`HGS_Data.GetTileByKey` _returnvalue (`HGS_ActorSnapComponent.TileKey` (`self.HGS_ActorSnap`))))
      (if _returnvalue_2
        (`TextRenderComponent.K2_SetText` (`self.HexCoordinate`) (`KismetTextLibrary.Conv_StringToText` (`HGS_Library.TileToSring` _outtile)))
        (`TextRenderComponent.K2_SetText` (`self.HexTileRefCount`) (`KismetTextLibrary.Conv_StringToText` (`KismetStringLibrary.Concat_StrStr` "RefCount: " (`KismetStringLibrary.Conv_IntToString` (`.RefCount` (break `HGS_Tile` _outtile))))))))))